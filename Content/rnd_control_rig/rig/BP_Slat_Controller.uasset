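; Controller actor that groups and rotates slat bones on a BP_Slat's Control Rig around its hinge controls.
; Construction script gathers hinge control names from the rig's bones.
; Update events build bone groups from column and row names, for one hinge or a six-column staggered cluster, then pass them to the rig and rebind.
; Timelines animate hinge pitch, with the cluster's main timeline triggering per-hinge timelines through event tracks.
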(event `UpdateBones`
  (`self.As BP Slat 0`
    (:`then`
      (`KismetArrayLibrary.Array_Clear` (`self.BoneGroup`))
      (if (not (> (`self.Hinge`) (`KismetArrayLibrary.Array_Length` (`.HingeName_8_037F781D4684CB2993B8F3B35C41F4A7` (break `/Game/HRLV_Sandbox/rnd_control_rig/rig/HingeStruct` (`self.Hingey`))))))
        (for _index (range (`self.StartRow`) (+ (`self.EndRow`) 1))
          (`KismetArrayLibrary.Array_Add` (`self.BoneGroup`) (`KismetStringLibrary.Conv_StringToName` (`KismetSystemLibrary.MakeLiteralString` (`KismetStringLibrary.Concat_StrStr` "0_" (`KismetStringLibrary.Conv_IntToString` (`self.TargetColumn`)) "_" (`KismetStringLibrary.Conv_IntToString` _index) "_geo")))))
        (`KismetArrayLibrary.Array_Set` (`.BoneGroup_9_681AD5434A16BF7320E5A4AABCBC4719` (break `/Game/HRLV_Sandbox/rnd_control_rig/rig/HingeStruct` (`self.Hingey`))) (`self.Hinge`) (make `/Game/HRLV_Sandbox/rnd_control_rig/rig/MullStruct` (`self.BoneGroup`)))
        (bind _asrnd_cr_mullion_zero_ctrl_rig (cast `/Game/HRLV_Sandbox/rnd_control_rig/rig/RND_CR_MullionZero_CtrlRig` (`ControlRigComponent.GetControlRig` (`/Game/HRLV_Sandbox/rnd_control_rig/rig/BP_Slat0.SlatControlRig` (`self.As BP Slat 0`)))))
        (set `/Game/HRLV_Sandbox/rnd_control_rig/rig/RND_CR_MullionZero_CtrlRig.Hingey` (`self.Hingey`) _asrnd_cr_mullion_zero_ctrl_rig)
        (`/Game/HRLV_Sandbox/rnd_control_rig/rig/BP_Slat0.Bind` (`self.As BP Slat 0`))))
    (:`else`)))

(event `UpdateRotation`
  (bind (_hingename _bonegroup) (break `/Game/HRLV_Sandbox/rnd_control_rig/rig/HingeStruct` (`self.Hingey`)))
  (bind _slatcontrolrig (`/Game/HRLV_Sandbox/rnd_control_rig/rig/BP_Slat0.SlatControlRig` (`self.As BP Slat 0`)))
  (bind _output (`|GetArrayItem` _hingename (`self.Hinge`)))
  (bind (_returnvalue_roll _returnvalue_pitch _returnvalue_yaw) (`KismetMathLibrary.BreakRotator` (`ControlRigComponent.GetControlRotator` _slatcontrolrig _output "LocalSpace")))
  (`self.As BP Slat 0`
    (:`then`
      (if (not (> (`self.Hinge`) (`KismetArrayLibrary.Array_Length` _bonegroup)))
        (bind (_direction _newtrack_0) (`Timeline|Timeline` :!via `PlayFromStart`)
          (:`Update`
            (`ControlRigComponent.SetControlRotator` _slatcontrolrig _output (`KismetMathLibrary.MakeRotator` _returnvalue_roll _newtrack_0 _returnvalue_yaw) "LocalSpace")))))
    (:`else`)))

(event `AttachBonesCluster`
  (`self.As BP Slat 0`
    (:`then`
      (`KismetArrayLibrary.Array_Clear` (`self.BoneGroup`))
      (if (not (> (`self.Hinge`) (`KismetArrayLibrary.Array_Length` (`.HingeName_8_037F781D4684CB2993B8F3B35C41F4A7` (break `/Game/HRLV_Sandbox/rnd_control_rig/rig/HingeStruct` (`self.Hingey`))))))
        (for _index (range 6)
          (for _index_2 (range (`self.StartRow`) (+ (- (`self.EndRow`) _index) 1))
            (`KismetArrayLibrary.Array_Add` (`self.BoneGroup`) (`KismetStringLibrary.Conv_StringToName` (`KismetSystemLibrary.MakeLiteralString` (`KismetStringLibrary.Concat_StrStr` "0_" (`KismetStringLibrary.Conv_IntToString` _index) "_" (`KismetStringLibrary.Conv_IntToString` _index_2) "_geo")))))
          (`KismetArrayLibrary.Array_Set` (`.BoneGroup_9_681AD5434A16BF7320E5A4AABCBC4719` (break `/Game/HRLV_Sandbox/rnd_control_rig/rig/HingeStruct` (`self.Hingey`))) _index (make `/Game/HRLV_Sandbox/rnd_control_rig/rig/MullStruct` (`self.BoneGroup`)))
          (`KismetArrayLibrary.Array_Clear` (`self.BoneGroup`))
          (bind _asrnd_cr_mullion_zero_ctrl_rig (cast `/Game/HRLV_Sandbox/rnd_control_rig/rig/RND_CR_MullionZero_CtrlRig` (`ControlRigComponent.GetControlRig` (`/Game/HRLV_Sandbox/rnd_control_rig/rig/BP_Slat0.SlatControlRig` (`self.As BP Slat 0`)))))
          (set `/Game/HRLV_Sandbox/rnd_control_rig/rig/RND_CR_MullionZero_CtrlRig.Hingey` (`self.Hingey`) _asrnd_cr_mullion_zero_ctrl_rig)
          (set `/Game/HRLV_Sandbox/rnd_control_rig/rig/RND_CR_MullionZero_CtrlRig.Offsets` (`|MakeArray` (0.0 10.0 0.0) (0.0 20.0 0.0) (0.0 30.0 0.0) (0.0 40.0 0.0) (0.0 50.0 0.0) (0.0 60.0 0.0) :!type "Vector Structure") _asrnd_cr_mullion_zero_ctrl_rig)
          (`/Game/HRLV_Sandbox/rnd_control_rig/rig/BP_Slat0.Bind` (`self.As BP Slat 0`)))))
    (:`else`)))

(event `RotationBoneCluster`
  (bind _slatcontrolrig (`/Game/HRLV_Sandbox/rnd_control_rig/rig/BP_Slat0.SlatControlRig` (`self.As BP Slat 0`)))
  (bind _slatcontrolrig_2 (`/Game/HRLV_Sandbox/rnd_control_rig/rig/BP_Slat0.SlatControlRig` (`self.As BP Slat 0`)))
  (bind _slatcontrolrig_3 (`/Game/HRLV_Sandbox/rnd_control_rig/rig/BP_Slat0.SlatControlRig` (`self.As BP Slat 0`)))
  (bind _slatcontrolrig_4 (`/Game/HRLV_Sandbox/rnd_control_rig/rig/BP_Slat0.SlatControlRig` (`self.As BP Slat 0`)))
  (bind _slatcontrolrig_5 (`/Game/HRLV_Sandbox/rnd_control_rig/rig/BP_Slat0.SlatControlRig` (`self.As BP Slat 0`)))
  (bind _slatcontrolrig_6 (`/Game/HRLV_Sandbox/rnd_control_rig/rig/BP_Slat0.SlatControlRig` (`self.As BP Slat 0`)))
  (bind _output (`|GetArrayItem` (`.HingeName_8_037F781D4684CB2993B8F3B35C41F4A7` (break `/Game/HRLV_Sandbox/rnd_control_rig/rig/HingeStruct` (`self.Hingey`)))))
  (bind _output_2 (`|GetArrayItem` (`.HingeName_8_037F781D4684CB2993B8F3B35C41F4A7` (break `/Game/HRLV_Sandbox/rnd_control_rig/rig/HingeStruct` (`self.Hingey`))) 5))
  (bind _output_3 (`|GetArrayItem` (`.HingeName_8_037F781D4684CB2993B8F3B35C41F4A7` (break `/Game/HRLV_Sandbox/rnd_control_rig/rig/HingeStruct` (`self.Hingey`))) 3))
  (bind _output_4 (`|GetArrayItem` (`.HingeName_8_037F781D4684CB2993B8F3B35C41F4A7` (break `/Game/HRLV_Sandbox/rnd_control_rig/rig/HingeStruct` (`self.Hingey`))) 1))
  (bind _output_5 (`|GetArrayItem` (`.HingeName_8_037F781D4684CB2993B8F3B35C41F4A7` (break `/Game/HRLV_Sandbox/rnd_control_rig/rig/HingeStruct` (`self.Hingey`))) 2))
  (bind _output_6 (`|GetArrayItem` (`.HingeName_8_037F781D4684CB2993B8F3B35C41F4A7` (break `/Game/HRLV_Sandbox/rnd_control_rig/rig/HingeStruct` (`self.Hingey`))) 4))
  (bind (_returnvalue_roll _returnvalue_pitch _returnvalue_yaw) (`KismetMathLibrary.BreakRotator` (`ControlRigComponent.GetControlRotator` _slatcontrolrig_2 _output "LocalSpace")))
  (bind (_returnvalue_roll_2 _returnvalue_pitch_2 _returnvalue_yaw_2) (`KismetMathLibrary.BreakRotator` (`ControlRigComponent.GetControlRotator` _slatcontrolrig_3 _output_3 "LocalSpace")))
  (bind (_returnvalue_roll_3 _returnvalue_pitch_3 _returnvalue_yaw_3) (`KismetMathLibrary.BreakRotator` (`ControlRigComponent.GetControlRotator` _slatcontrolrig_4 _output_4 "LocalSpace")))
  (bind (_returnvalue_roll_4 _returnvalue_pitch_4 _returnvalue_yaw_4) (`KismetMathLibrary.BreakRotator` (`ControlRigComponent.GetControlRotator` _slatcontrolrig_5 _output_5 "LocalSpace")))
  (bind (_returnvalue_roll_5 _returnvalue_pitch_5 _returnvalue_yaw_5) (`KismetMathLibrary.BreakRotator` (`ControlRigComponent.GetControlRotator` _slatcontrolrig_6 _output_6 "LocalSpace")))
  (bind (_returnvalue_roll_6 _returnvalue_pitch_6 _returnvalue_yaw_6) (`KismetMathLibrary.BreakRotator` (`ControlRigComponent.GetControlRotator` _slatcontrolrig _output_2 "LocalSpace")))
  (`self.As BP Slat 0`
    (:`then`
      (bind (_direction _newtrack_0) (`Timeline|Timeline_0` :!via `PlayFromStart`)
        (:`Update`
          (`ControlRigComponent.SetControlRotator` _slatcontrolrig_2 _output (`KismetMathLibrary.MakeRotator` _returnvalue_roll _newtrack_0 _returnvalue_yaw) "LocalSpace"))
        (:`NewTrack_1`
          (bind (_direction_2 _newtrack_0_2) (`Timeline|Timeline_1` :!via `PlayFromStart`)
            (:`Update`
              (`ControlRigComponent.SetControlRotator` _slatcontrolrig_4 _output_4 (`KismetMathLibrary.MakeRotator` _returnvalue_roll_3 _newtrack_0_2 _returnvalue_yaw_3) "LocalSpace"))))
        (:`NewTrack_2`
          (bind (_direction_3 _newtrack_0_3) (`Timeline|Timeline_2` :!via `PlayFromStart`)
            (:`Update`
              (`ControlRigComponent.SetControlRotator` _slatcontrolrig_5 _output_5 (`KismetMathLibrary.MakeRotator` _returnvalue_roll_4 _newtrack_0_3 _returnvalue_yaw_4) "LocalSpace"))))
        (:`NewTrack_3`
          (bind (_direction_4 _newtrack_0_4) (`Timeline|Timeline_3` :!via `PlayFromStart`)
            (:`Update`
              (`ControlRigComponent.SetControlRotator` _slatcontrolrig_3 _output_3 (`KismetMathLibrary.MakeRotator` _returnvalue_roll_2 _newtrack_0_4 _returnvalue_yaw_2) "LocalSpace"))))
        (:`NewTrack_4`
          (bind (_direction_5 _newtrack_0_5) (`Timeline|Timeline_4` :!via `PlayFromStart`)
            (:`Update`
              (`ControlRigComponent.SetControlRotator` _slatcontrolrig_6 _output_6 (`KismetMathLibrary.MakeRotator` _returnvalue_roll_5 _newtrack_0_5 _returnvalue_yaw_5) "LocalSpace"))))
        (:`NewTrack_5`
          (bind (_direction_6 _newtrack_0_6) (`Timeline|Timeline_5` :!via `PlayFromStart`)
            (:`Update`
              (`ControlRigComponent.SetControlRotator` _slatcontrolrig _output_2 (`KismetMathLibrary.MakeRotator` _returnvalue_roll_6 _newtrack_0_6 _returnvalue_yaw_6) "LocalSpace"))))))
    (:`else`)))

(fn `UserConstructionScript`
  (bind (_hingename _bonegroup) (break `/Game/HRLV_Sandbox/rnd_control_rig/rig/HingeStruct` (`self.Hingey`)))
  (bind (_hingename_2 _bonegroup_2) (break `/Game/HRLV_Sandbox/rnd_control_rig/rig/HingeStruct` (`self.Hingey`)))
  (`KismetArrayLibrary.Array_Clear` _hingename_2)
  (`KismetArrayLibrary.Array_Clear` _bonegroup_2)
  (if (== (`KismetArrayLibrary.Array_Length` _hingename_2) 0)
    (bind _as_bp_slat_0 (`self.As BP Slat 0`)
      (:`then`
        (for _array_element (`ControlRigComponent.GetElementNames` (`/Game/HRLV_Sandbox/rnd_control_rig/rig/BP_Slat0.SlatControlRig` _as_bp_slat_0) "Bone")
          (bind _returnvalue (`KismetStringLibrary.Conv_NameToString` _array_element))
          (if (and (`KismetStringLibrary.Contains` _returnvalue "_hinge") (`KismetStringLibrary.NotEqual_StrStr` (`KismetStringLibrary.Conv_NameToString` _array_element) "cog_hinge"))
            (`KismetArrayLibrary.Array_Add` _hingename (`KismetStringLibrary.Conv_StringToName` (`KismetStringLibrary.Concat_StrStr` _returnvalue "_ctrl")))
            (`KismetArrayLibrary.Array_Add` _bonegroup (make `/Game/HRLV_Sandbox/rnd_control_rig/rig/MullStruct` (`|MakeArray` "None" :!type "Name"))))))
      (:`else`))))